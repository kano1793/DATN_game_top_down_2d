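; Level manager that runs a timed survival run: enemy waves, bosses, music changes and an opening random buff display.
; A one-second timer calls the function named after the elapsed second, so numbered functions script the level timeline.
; These trigger continuous refills, bursts, formation spawners or unpooled large enemies; bullets, regular mobs and pickups reuse pooled actors.
; It also converts kills, time and level into score and saved coins.
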(event `self.ReceiveTick`
  (params (DeltaSeconds :type "Float (single-precision)"))
  ;[0.1528 1 0] Test
)

(event `self.ReceiveBeginPlay`
  ;[0 0 0] Initialization
  (set `/Game/_SG/Data/GI_SG.Ref_LevelManager` self (`/Game/_SG/Data/Flib_SG.Flib_GetGI`))
  (bind _returnvalue (`KismetSystemLibrary.K2_SetTimerDelegate` (delegate `TimeCount`) 1.0 true))
  (set `self.TimerHandle_Level` _returnvalue)
  (if (`KismetSystemLibrary.IsValid` (`/Game/_SG/Data/Flib_SG.Flib_GetLayout`)) :!label _label
    (`self.RandomEvent`)
    (else
      (`KismetSystemLibrary.Delay` 0.02)
      (goto _label))))

(event `TimeCount`
  ;[0 0 0] Initialization
  (bind _result (`/Engine/EditorBlueprintResources/StandardMacros.IncrementInt` (`self.PlayGameTimer`))
    (:`  `
      (`/Game/_SG/Blueprints/UI/UI_Layout.UpdateTime` (`/Game/_SG/Data/PC_InGame.UI_Layout` (`/Game/_SG/Data/GI_SG.Ref_PCInGame` (`/Game/_SG/Data/Flib_SG.Flib_GetGI`))) (mod _result 60) (/ _result 60))
      (`KismetSystemLibrary.K2_SetTimer` null (`KismetStringLibrary.Conv_IntToString` (`self.PlayGameTimer`)) 0.05))))

(fn `1`
  (`/Game/_SG/Data/GI_SG.BGMManagement` (`/Game/_SG/Data/Flib_SG.Flib_GetGI`) "/Game/_SG/Assets/SFX/Musics/Cue_Normal.Cue_Normal"))

(fn `10`
  (`self.MobBurst` (`|MakeArray` 1) 6))

(fn `1000`
  (`self.UnpoolingMobs` 26 (3.0 3.0 3.0))
  (`self.ContinuousMobs` 100 (`|MakeArray` 27)))

(fn `101`
  (`self.MobBurst` (`|MakeArray` 1) 20)
  (`self.MobBurst` (`|MakeArray` 2) 20)
  (`self.ContinuousMobs` 35 (`|MakeArray` 1 2)))

(fn `1030`
  (`self.MobPatterns` "NewEnumerator3" 1 510)
  (`self.MobBurst` (`|MakeArray` 280) 1)
  (`self.MobBurst` (`|MakeArray` 290) 1))

(fn `1050`
  (`self.MobPatterns` "NewEnumerator3" 5 510))

(fn `1090`
  (`self.ContinuousMobs` 100 (`|MakeArray` 28 29)))

(fn `120`
  (`self.UnpoolingMobs` 3 (3.0 3.0 3.0)))

(fn `1200`
  (`self.MobAllDie`))

(fn `1205`
  ;[0 0 0] Spawn last boss
  (`self.UnpoolingMobs` 31 (4.0 4.0 4.0))
  (`/Game/_SG/Data/GI_SG.BGMManagement` (`/Game/_SG/Data/Flib_SG.Flib_GetGI`) "/Game/_SG/Assets/SFX/Musics/Cue_BOSS.Cue_BOSS"))

(fn `1215`
  (`self.ContinuousMobs` 40 (`|MakeArray` 30)))

(fn `125`
  (`self.ContinuousMobs` 45 (`|MakeArray` 2 1)))

(fn `140`
  (`self.MobPatterns` "NewEnumerator3" 1 501))

(fn `1500`
  (`self.MobBurst` (`|MakeArray` 30) 40))

(fn `180`
  (`self.ContinuousMobs` 30 (`|MakeArray` 2 4)))

(fn `2`
  (`self.ContinuousMobs` 8 (`|MakeArray` 1)))

(fn `200`
  (`self.MobPatterns` "NewEnumerator2" 0 502)
  (`self.ContinuousMobs` 40 (`|MakeArray` 4)))

(fn `220`
  (`self.MobPatterns` "NewEnumerator3" 5 501)
  (`self.ContinuousMobs` 55 (`|MakeArray` 4 2)))

(fn `240`
  (`self.MobPatterns` "NewEnumerator3" 5 502))

(fn `260`
  (`self.ContinuousMobs` 40 (`|MakeArray` 2 4 5))
  (`self.UnpoolingMobs` 6 (3.0 3.0 3.0)))

(fn `280`
  (`self.MobPatterns` "NewEnumerator1" 0 502)
  (`self.ContinuousMobs` 40 (`|MakeArray` 4 5)))

(fn `300`
  (`self.MobPatterns` "NewEnumerator3" 10 502))

(fn `315`
  (`self.ContinuousMobs` 60 (`|MakeArray` 7 8 9)))

(fn `340`
  (`self.ContinuousMobs` 40 (`|MakeArray` 7))
  (`self.MobPatterns` "NewEnumerator2" 0 503))

(fn `35`
  (`self.ContinuousMobs` 35 (`|MakeArray` 1 2)))

(fn `360`
  (`self.ContinuousMobs` 60 (`|MakeArray` 7 10))
  (`self.MobPatterns` "NewEnumerator3" 5 503))

(fn `370`
  (`self.UnpoolingMobs` 11 (3.0 3.0 3.0))
  (`self.ContinuousMobs` 60 (`|MakeArray` 7 10 8 9)))

(fn `390`
  (`self.ContinuousMobs` 50 (`|MakeArray` 7 10 8 9 12)))

(fn `425`
  (`self.MobPatterns` "NewEnumerator2" 5 503)
  (`self.ContinuousMobs` 40 (`|MakeArray` 10 12)))

(fn `45`
  (`self.MobPatterns` "NewEnumerator1" 0 2))

(fn `455`
  (`self.MobPatterns` "NewEnumerator1" 0 504)
  (`self.ContinuousMobs` 75 (`|MakeArray` 10 12 13)))

(fn `460`
  (`self.MobPatterns` "NewEnumerator2" 0 505))

(fn `480`
  (`self.UnpoolingMobs` 14 (3.0 3.0 3.0)))

(fn `50`
  (`self.MobBurst` (`|MakeArray` 1 2) 15))

(fn `500`
  (`self.MobPatterns` "NewEnumerator3" 3 504))

(fn `505`
  (`self.MobPatterns` "NewEnumerator3" 3 505))

(fn `520`
  (`self.MobBurst` (`|MakeArray` 15) 5))

(fn `540`
  (`self.ContinuousMobs` 55 (`|MakeArray` 12 13 15)))

(fn `580`
  (`self.MobPatterns` "NewEnumerator3" 10 506))

(fn `60`
  (`self.MobBurst` (`|MakeArray` 1) 10))

(fn `620`
  (`self.UnpoolingMobs` 16 (4.0 4.0 4.0))
  (`/Game/_SG/Data/GI_SG.BGMManagement` (`/Game/_SG/Data/Flib_SG.Flib_GetGI`) "/Game/_SG/Assets/SFX/Musics/Cue_BOSS.Cue_BOSS"))

(fn `65`
  (`self.MobPatterns` "NewEnumerator2" 0 1))

(fn `650`
  (`self.ContinuousMobs` 55 (`|MakeArray` 15 17))
  (`self.MobBurst` (`|MakeArray` 17) 40))

(fn `690`
  (`self.MobPatterns` "NewEnumerator3" 5 507)
  (`self.ContinuousMobs` 75 (`|MakeArray` 18 17)))

(fn `720`
  (`self.MobPatterns` "NewEnumerator2" 0 507)
  (`self.ContinuousMobs` 55 (`|MakeArray` 18 17)))

(fn `750`
  (`self.ContinuousMobs` 85 (`|MakeArray` 18 20)))

(fn `790`
  (`self.MobPatterns` "NewEnumerator3" 20 507)
  (`/Game/_SG/Data/GI_SG.BGMManagement` (`/Game/_SG/Data/Flib_SG.Flib_GetGI`) "/Game/_SG/Assets/SFX/Musics/Cue_Normal.Cue_Normal"))

(fn `820`
  (`self.UnpoolingMobs` 19 (3.0 3.0 3.0))
  (`self.ContinuousMobs` 75 (`|MakeArray` 17 20)))

(fn `840`
  (`self.ContinuousMobs` 75 (`|MakeArray` 21 24)))

(fn `85`
  (`self.ContinuousMobs` 35 (`|MakeArray` 2)))

(fn `865`
  (`self.MobPatterns` "NewEnumerator2" 0 508)
  (`self.MobBurst` (`|MakeArray` 21 24) 25))

(fn `900`
  (`self.UnpoolingMobs` 22 (3.0 3.0 3.0))
  (`self.UnpoolingMobs` 23 (3.0 3.0 3.0))
  (`self.ContinuousMobs` 75 (`|MakeArray` 24))
  (`self.MobBurst` (`|MakeArray` 24) 25))

(fn `95`
  (`self.MobPatterns` "NewEnumerator3" 3 501))

(fn `950`
  (`self.ContinuousMobs` 75 (`|MakeArray` 24 25))
  (`self.MobPatterns` "NewEnumerator1" 0 509))

(fn `955`
  (`self.MobPatterns` "NewEnumerator2" 0 509))

(fn `960`
  (`self.MobPatterns` "NewEnumerator2" 0 509))

(fn `CalculateCoins`
  (params (FinalScore :type Integer))
  (locals (L_Incremental :type Integer :default 0))
  (bind _output_get (set `local.L_Incremental` (`KismetMathLibrary.FTrunc` (/ (`KismetMathLibrary.Conv_IntToDouble` FinalScore) (`KismetMathLibrary.RandomFloatInRange` 9.0 10.0)))))
  (bind _finalcoin (`/Game/_SG/Data/GI_SG.AddCoins` (`/Game/_SG/Data/Flib_SG.Flib_GetGI`) _output_get))
  (`self.SaveCoinData`)
  (`/Game/_SG/Blueprints/UI/UI_Layout.UpdateGameOverUI` (`/Game/_SG/Data/Flib_SG.Flib_GetLayout`) (`self.FinalScore`) _finalcoin))

(fn `CalculateScores`
  (bind _ref_player (`/Game/_SG/Data/GI_SG.Ref_Player` (`/Game/_SG/Data/Flib_SG.Flib_GetGI`)))
  (bind _output_get (set `self.FinalScore` (+ (* (`/Game/_SG/Blueprints/BP_Player.Killings` _ref_player) 50) (* (`self.PlayGameTimer`) 10) (* (`.CurLevel_2_F85C10F54231D7455B1C48B8C61A8134` (break `/Game/_SG/Blueprints/Structs/F_PlayerInfo` (`/Game/_SG/Blueprints/BP_Player.PlayerAttributes` _ref_player))) 100))))
  (`self.CalculateCoins` _output_get))

(fn `ClearTimer`
  (`KismetSystemLibrary.K2_ClearAndInvalidateTimerHandle` (`self.Timer_TryRespawningMoreMobs`))
  (`KismetSystemLibrary.K2_ClearAndInvalidateTimerHandle` (`self.TimerHandle_Level`)))

(fn `ContinuousMobs`
  (params (AllowActiveMobNums :type Integer) (AllowMobsID :type "Array of Integer"))
  (set `self.Allow Active Mob Nums` AllowActiveMobNums) ; How many enemies are allowed to pursue player character at the same time?
  (`KismetArrayLibrary.Array_Clear` (`self.AllowMobsID`))
  (set `self.AllowMobsID` AllowMobsID)
  (for _ (range (`self.Allow Active Mob Nums`))
    (`self.PoolingMobs` true 0 (0.0 0.0 0.0) true) ; Check "random?" and "MoveToPlayer" booleans
  )
  (`KismetSystemLibrary.K2_ClearAndInvalidateTimerHandle` (`self.Timer_TryRespawningMoreMobs`))
  (bind _returnvalue (`KismetSystemLibrary.K2_SetTimer` null "TryRespawnMoreMobs" 0.2 true)) ; Checking whether more mobs are allowed every 0.2 seconds
  (set `self.Timer_TryRespawningMoreMobs` _returnvalue))

(fn `MobAllDie`
  (`self.ContinuousMobs` 0 (`|MakeArray` 0)) ; Limitation set to 0
  (bind _outactors (`GameplayStatics.GetAllActorsOfClass` "/Game/_SG/Blueprints/BP_AI.BP_AI_C"))
  (for _array_element _outactors
    (`/Game/_SG/Blueprints/BP_AI.ForceDeath` _array_element)))

(fn `MobBurst`
  (params (AllowMobsID :type "Array of Integer") (RepeatedLoops :type Integer))
  (`KismetArrayLibrary.Array_Clear` (`self.AllowMobsID`))
  (set `self.AllowMobsID` AllowMobsID)
  (for _ (range (+ RepeatedLoops 1))
    (`self.PoolingMobs` true 0 (0.0 0.0 0.0) true) ; Tick "Random?" and "Move to Player" !
  ))

(fn `MobPatterns`
  (params (Pattern :type "/Game/_SG/Blueprints/Enumerations/E_PatternTypes Enum" :default "NewEnumerator0") (MaxLoop :type Integer) (SpecifiedID :type Integer))
  (bind _returnvalue (`self.K2_GetActorLocation` (`/Game/_SG/Data/GI_SG.Ref_Player` (`/Game/_SG/Data/Flib_SG.Flib_GetGI`))))
  (switch `/Game/_SG/Blueprints/Enumerations/E_PatternTypes` Pattern
    (:`NewEnumerator1`
      (`|SpawnActorFromClass` "/Game/_SG/Blueprints/BPA/Patterns/BPA_Cross.BPA_Cross_C" (`KismetMathLibrary.MakeTransform` _returnvalue) "Undefined" "MultiplyWithRoot" null (`local.SpecifiedID`) null))
    (:`NewEnumerator2`
      (`|SpawnActorFromClass` "/Game/_SG/Blueprints/BPA/Patterns/BPA_Circle.BPA_Circle_C" (`KismetMathLibrary.MakeTransform` _returnvalue) "Undefined" "MultiplyWithRoot" null (`local.SpecifiedID`) null))
    (:`NewEnumerator3`
      (`|SpawnActorFromClass` "/Game/_SG/Blueprints/BPA/Patterns/BPA_Grid.BPA_Grid_C" (`KismetMathLibrary.MakeTransform` (`self.K2_GetActorLocation` (`/Game/_SG/Data/GI_SG.Ref_Player` (`/Game/_SG/Data/Flib_SG.Flib_GetGI`)))) "Undefined" "MultiplyWithRoot" null MaxLoop (`local.SpecifiedID`) null))))

(fn `PoolingBullets`
  (params (Location :type "Vector Structure") (OverallScale :type "Vector Structure") (Damage :type "Float (double-precision)") (ProjectileVelocity :type "Vector Structure") (TargetTag :type Name) (DamageCauser :type "Actor Object Reference") (NewFlipbook :type "PaperFlipbook Object Reference") (FlipbookScale :type "Vector Structure") (LifeSpan :type "Float (double-precision)") (FlipbookRotation :type "Rotator Structure" :default (struct :`Yaw` -180.0 :`Roll` -90.0)))
  (locals (L_AvailableBullet :type "/Game/_SG/Blueprints/BPA/BPA_Bullet Object Reference"))
  (bind _l_availablebullet (`local.L_AvailableBullet`))
  (for _array_element (`self.BulletPool`)
    (if (`|EnumEquality` (`/Game/_SG/Blueprints/BPA/BPA_Bullet.BulletState` _array_element) "NewEnumerator1")
      (set `local.L_AvailableBullet` _array_element)
      (break)))
  (`local.L_AvailableBullet`
    (:`then`
      _)
    (:`else`
      (bind _returnvalue (`|SpawnActorFromClass` "/Game/_SG/Blueprints/BPA/BPA_Bullet.BPA_Bullet_C" (`KismetMathLibrary.MakeTransform` (0.0 1000.0 -10000.0)) "AdjustIfPossibleButAlwaysSpawn" "MultiplyWithRoot" null "None" null)) ; Spawn a new bullet instance when all exsited bullets are occupied.
      (bind _output_get (set `local.L_AvailableBullet` _returnvalue))
      (`KismetArrayLibrary.Array_Add` (`self.BulletPool`) _output_get)))
  (`/Game/_SG/Blueprints/BPA/BPA_Bullet.SetupBulletProperties` _l_availablebullet (`local.OverallScale`) (`local.Damage`) (`local.ProjectileVelocity`) (`local.TargetTag`) (`local.DamageCauser`) (`local.NewFlipbook`) (`local.FlipbookScale`) LifeSpan (`local.FlipbookRotation`))
  (`self.K2_SetActorLocation` _l_availablebullet (`local.Location`) false false) ; After setup/initializing new bullet settings, teleport it to desired position.
)

(fn `PoolingMobs`
  (params (`Random?` :type Boolean) (ID :type Integer) (SpecifiedLocation :type "Vector Structure") (`MoveToPlayer?` :type Boolean) (Destination :type "Vector Structure"))
  (locals (L_Mob :type "/Game/_SG/Blueprints/BP_AI Object Reference"))
  (bind _allowmobsid (`self.AllowMobsID`))
  (for _array_element (`self.TotalMobPool`)
    (if (`|EnumEquality` (`/Game/_SG/Blueprints/BP_AI.MobState` _array_element) "NewEnumerator2")
      (set `local.L_Mob` _array_element)
      (break)))
  (`local.L_Mob`
    (:`then`
      _)
    (:`else`
      (bind _returnvalue (`|SpawnActorFromClass` "/Game/_SG/Blueprints/BP_AI.BP_AI_C" (`KismetMathLibrary.MakeTransform` (0.0 0.0 -10000.0)) "Undefined" "MultiplyWithRoot" null true null))
      (bind _output_get (set `local.L_Mob` _returnvalue))
      (`KismetArrayLibrary.Array_AddUnique` (`self.TotalMobPool`) _output_get)))
  (set `/Game/_SG/Blueprints/BP_AI.MobState` "NewEnumerator3" (`local.L_Mob`))
  (if (`local.Random?`)
    (`KismetArrayLibrary.Array_Add` (`self.ActiveMobPool`) (`local.L_Mob`))
    (`KismetArrayLibrary.Array_Shuffle` _allowmobsid)
    (`/Game/_SG/Blueprints/BP_AI.SpawnSetup` (`local.L_Mob`) (`KismetStringLibrary.Conv_StringToName` (`KismetStringLibrary.Conv_IntToString` (`|GetArrayItem` _allowmobsid))) true (0.0 0.0 0.0) true (0.0 0.0 0.0))
    (else
      (`/Game/_SG/Blueprints/BP_AI.SpawnSetup` (`local.L_Mob`) (`KismetStringLibrary.Conv_StringToName` (`KismetStringLibrary.Conv_IntToString` (`local.ID`))) false (`local.SpecifiedLocation`) (`local.MoveToPlayer?`) (`local.Destination`)))))

(fn `PoolingPickupBase`
  (params (PickupType :type "/Game/_SG/Blueprints/Enumerations/E_PickupTypes Enum" :default "NewEnumerator0") (Location :type "Vector Structure") (EXP :type "Float (double-precision)"))
  (locals (L_Pickup :type "/Game/_SG/Blueprints/BPA/BPA_Pickup Object Reference"))
  (bind _l_pickup (`local.L_Pickup`))
  (for _array_element (`self.PickupPool`)
    (if (`|EnumEquality` (`/Game/_SG/Blueprints/BPA/BPA_Pickup.PickupState` _array_element) "NewEnumerator3")
      (set `local.L_Pickup` _array_element)
      (break)))
  (`local.L_Pickup`
    (:`then`
      _)
    (:`else`
      (bind _returnvalue (`|SpawnActorFromClass` "/Game/_SG/Blueprints/BPA/BPA_Pickup.BPA_Pickup_C" (`KismetMathLibrary.MakeTransform` (1000.0 0.0 -10000.0)) "AdjustIfPossibleButAlwaysSpawn" "MultiplyWithRoot" null "NewEnumerator1" null))
      (bind _output_get (set `local.L_Pickup` _returnvalue))
      (`KismetArrayLibrary.Array_AddUnique` (`self.PickupPool`) _output_get)))
  (`/Game/_SG/Blueprints/BPA/BPA_Pickup.SetupPickupInst` _l_pickup (`local.PickupType`) (`local.EXP`))
  (`self.K2_SetActorLocation` _l_pickup (`local.Location`) false false) ; Simply teleport actor as a whole, not adjust paper sprite independently anymore here
)

(fn `RandomEvent`
  (locals (L_Title :type Text) (L_Result :type Integer) (L_MultiplierPerLevel :type Integer))
  (bind _gi (`/Game/_SG/Data/Flib_SG.Flib_GetGI`))
  (bind _randomevents (`self.RandomEvents`))
  (bind _ref_randomeffect (`/Game/_SG/Data/GI_SG.Ref_RandomEffect` (`/Game/_SG/Data/Flib_SG.Flib_GetGI`)))
  (`WidgetSwitcher.SetActiveWidgetIndex` (`/Game/_SG/Blueprints/UI/UI_Layout.WS_InGame` (`/Game/_SG/Data/Flib_SG.Flib_GetLayout`)) 2)
  (`KismetArrayLibrary.Array_Shuffle` _randomevents)
  (set `/Game/_SG/Data/GI_SG.Ref_RandomEffect` (`|GetArrayItem` _randomevents) _gi)
  (for _array_element (`/Game/_SG/Data/GI_SG.Shop Item Info` _gi)
    (bind (_displayname _currentlv _maxlv _icon _nextcost _upgradetag) (break `/Game/_SG/Blueprints/Structs/F_ShopItemInfo` _array_element))
    (if (`KismetStringLibrary.EqualEqual_StrStr` _upgradetag _ref_randomeffect)
      (switch `string` _ref_randomeffect
        (:`rss_randomatk`
          (set `local.L_Title` "ATK")
          (set `local.L_MultiplierPerLevel` 3))
        (:`rss_randomcritprobability`
          (set `local.L_Title` "Critical probability")
          (set `local.L_MultiplierPerLevel` 2))
        (:`rss_randompickup`
          (set `local.L_Title` "Pickup radius")
          (set `local.L_MultiplierPerLevel` 3))
        (:`rss_randomspd`
          (set `local.L_Title` "Moving speed")
          (set `local.L_MultiplierPerLevel` 2))
        (:`rss_randomdef`
          (set `local.L_Title` "Defence")
          (set `local.L_MultiplierPerLevel` 2)))
      (set `local.L_Result` (* (`local.L_MultiplierPerLevel`) _currentlv))
      (`/Game/_SG/Blueprints/UI/UI_Layout.InitRandomBuff` (`/Game/_SG/Data/Flib_SG.Flib_GetLayout`) _icon (select `bool` (== _currentlv 0) :`false` (`|FormatText` "{a} is increased by {b}%." (`local.L_Title`) (`local.L_Result`)) :`true` "No effects") _displayname (`KismetTextLibrary.Conv_IntToText` _currentlv false false)))))

(fn `SaveCoinData`
  (bind _gi (`/Game/_SG/Data/Flib_SG.Flib_GetGI`))
  (bind _ref_savegameplay (`/Game/_SG/Data/GI_SG.Ref_SaveGameplay` _gi))
  (set `/Game/_SG/Data/Saves/GSave_Gameplay.Coins` (`/Game/_SG/Data/GI_SG.Coins` _gi) _ref_savegameplay)
  (`GameplayStatics.SaveGameToSlot` _ref_savegameplay (`/Game/_SG/Data/GI_SG.SaveSlots` _gi)))

(fn `TryRespawnMoreMobs`
  (if (< (`KismetArrayLibrary.Array_Length` (`self.ActiveMobPool`)) (`self.Allow Active Mob Nums`))
    (`self.PoolingMobs` true 0 (0.0 0.0 0.0) true)))

(fn `UnpoolingMobs`
  (params (ID :type Integer) (Scale :type "Vector Structure"))
  (bind _returnvalue (`|SpawnActorFromClass` "/Game/_SG/Blueprints/BP_AI.BP_AI_C" (`KismetMathLibrary.MakeTransform` (0.0 0.0 -9990.0) (struct) Scale) "Undefined" "MultiplyWithRoot" null false null))
  (`/Game/_SG/Blueprints/BP_AI.SpawnSetup` _returnvalue (`KismetStringLibrary.Conv_StringToName` (`KismetStringLibrary.Conv_IntToString` ID)) true (0.0 0.0 0.0) true (0.0 0.0 0.0)) ; IMPORTANT: tick "Random Location" and "Move to Player?"
)

(fn `UserConstructionScript`)
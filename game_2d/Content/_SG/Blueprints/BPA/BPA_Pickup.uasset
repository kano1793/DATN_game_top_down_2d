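; BPA_Pickup is a pooled pickup actor for EXP and magnet items, with its sprite chosen by type.
; A tagged player overlapping the sphere starts a timeline that pulls it in at fixed height, with a counter that skips repeated transitions.
; On arrival, ItemEffect plays sound and messages the player, then the actor hides off-map and resets after a delay.
; Setup randomizes sprite height slightly to reduce flicker.
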(event `self.Sphere.OnComponentBeginOverlap`
  (params (OverlappedComponent :type "PrimitiveComponent Object Reference") (OtherActor :type "Actor Object Reference") (OtherComp :type "PrimitiveComponent Object Reference") (OtherBodyIndex :type Integer) (bFromSweep :type Boolean) (SweepResult :type "HitResult Structure (by ref)"))
  ;[0 0 0] Start transitional movement
  (if (and (`self.ActorHasTag` OtherActor "player") (`|EnumEquality` (`self.PickupState`) "NewEnumerator1"))
    (set `self.ReferenceActor` OtherActor)
    (set `self.PickupState` "NewEnumerator2")
    (bind _result (`/Engine/EditorBlueprintResources/StandardMacros.IncrementInt` (`self.AvoidLooping`))
      (:`  `
        (if (<= _result 4)
          (`Timeline|MagnetMovement` :!via `PlayFromStart`
            (:`Update`
              (bind _referenceactor (`self.ReferenceActor`)
                (:`then`
                  (`PrimitiveComponent.SetCollisionResponseToChannel` (`self.Capsule`) "ECC_Pawn" "ECR_Overlap")
                  (bind (_returnvalue_x _returnvalue_y) (`KismetMathLibrary.BreakVector` (`KismetMathLibrary.VInterpTo` (`self.K2_GetActorLocation`) (`self.K2_GetActorLocation` _referenceactor) (`GameplayStatics.GetWorldDeltaSeconds`) 5.0)))
                  (`self.K2_SetActorLocation` (`KismetMathLibrary.MakeVector` _returnvalue_x _returnvalue_y 17.0))
                  (if (<= (`self.GetDistanceTo` (`self.ReferenceActor`) self) 20.0)
                    (`self.ItemEffect` (`self.ReferenceActor`) :!label _label)
                    (`TimelineComponent.Stop` (`self.MagnetMovement`))
                    (`self.ReturnToPool`)))
                (:`else`))))
          (else
            (`self.SkipTransition`)))))))

(event `SkipTransition`
  ;[0 0 0] Start transitional movement
  (goto _label))

(event `ReturnToPool`
  ;[0 0 0] Return to pool
  (set `self.ReferenceActor` null)
  (`PrimitiveComponent.SetCollisionResponseToChannel` (`self.Sphere`) "ECC_GameTraceChannel1" "ECR_Ignore")
  (`PrimitiveComponent.SetCollisionResponseToChannel` (`self.Capsule`) "ECC_Pawn" "ECR_Ignore")
  (`self.SetActorHiddenInGame` true)
  (`self.K2_SetActorLocation` (1000.0 0.0 -10000.0)) ; Teleport to origin first
  ;;[1 0 0] Cool down interval
  (`KismetSystemLibrary.Delay` 1.0)
  (set `self.AvoidLooping` 0) ; Reset
  (`PrimitiveComponent.SetCollisionResponseToChannel` (`self.Sphere`) "ECC_GameTraceChannel1" "ECR_Overlap")
  (`PrimitiveComponent.SetCollisionResponseToChannel` (`self.Capsule`) "ECC_Pawn" "ECR_Overlap")
  (`self.SetActorHiddenInGame` false)
  (set `self.PickupState` "NewEnumerator3"))

(event `SetupPickupInst`
  (params (Type :type "/Game/_SG/Blueprints/Enumerations/E_PickupTypes Enum" :default "NewEnumerator0") (EXPValue :type "Float (double-precision)"))
  ;[0 0 0] Setup Pickup Base Instance
  (bind _output_get (set `self.PickupType` Type))
  (set `self.EXPValue` EXPValue)
  (`PaperSpriteComponent.SetSprite` (`self.PaperSprite`) (select `/Game/_SG/Blueprints/Enumerations/E_PickupTypes` _output_get :`NewEnumerator1` "/Game/_SG/Assets/Icons/Sprite_EXP_01.Sprite_EXP_01" :`NewEnumerator2` "/Game/_SG/Assets/Icons/Sprite_EXP_02.Sprite_EXP_02" :`NewEnumerator3` "/Game/_SG/Assets/Icons/Sprite_Magnet.Sprite_Magnet" :!type "PaperSprite Object Reference"))
  (`self.AvoidFlicking`) ; We adjust paper sprite world location height when it is in the pool, so the base height is -10000
  (set `self.PickupState` "NewEnumerator1"))

(fn `AvoidFlicking`
  (bind (_returnvalue_x _returnvalue_y) (`KismetMathLibrary.BreakVector` (`SceneComponent.K2_GetComponentLocation` (`self.PaperSprite`))))
  (`SceneComponent.K2_SetWorldLocation` (`self.PaperSprite`) (`KismetMathLibrary.MakeVector` _returnvalue_x _returnvalue_y (+ -10000.0 (`KismetMathLibrary.RandomFloatInRange` 1.0 3.0))) false false))

(fn `ItemEffect`
  (params (Target :type "Actor Object Reference"))
  (`/Engine/EditorBlueprintResources/StandardMacros.IsValid` Target
    (:`Is Valid`
      (switch `/Game/_SG/Blueprints/Enumerations/E_PickupTypes` (`self.PickupType`)
        (:`NewEnumerator1`
          (`/Game/_SG/Data/GI_SG.CoinSound` (`/Game/_SG/Data/Flib_SG.Flib_GetGI`))
          (message `/Game/_SG/Blueprints/Interfaces/BPI_Interaction.INT_AddEXP` (`local.Target`) (`KismetMathLibrary.FTrunc` (`self.EXPValue`))))
        (:`NewEnumerator3`
          (`GameplayStatics.SpawnSoundAtLocation` "/Game/Interface_And_Item_Sounds/Cues/Bar_Filling_01_Cue.Bar_Filling_01_Cue" (`self.K2_GetActorLocation`) (struct) 1.0 1.0 0.0 null null)
          (message `/Game/_SG/Blueprints/Interfaces/BPI_Interaction.INT_TriggerMagnet` (`local.Target`)))))))

(fn `UserConstructionScript`
  (`PaperSpriteComponent.SetSprite` (`self.PaperSprite`) (select `/Game/_SG/Blueprints/Enumerations/E_PickupTypes` (`self.PickupType`) :`NewEnumerator1` "/Game/_SG/Assets/Icons/Sprite_EXP_01.Sprite_EXP_01" :`NewEnumerator2` "/Game/_SG/Assets/Icons/Sprite_EXP_02.Sprite_EXP_02" :`NewEnumerator3` "/Game/_SG/Assets/Icons/Sprite_Magnet.Sprite_Magnet" :!type "PaperSprite Object Reference")))
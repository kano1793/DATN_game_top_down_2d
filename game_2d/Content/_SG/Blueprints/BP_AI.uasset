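; Base pooled Paper2D enemy that chases the player or walks to a destination, deals repeating touch damage, and drops EXP or occasional other pickups.
; SpawnSetup loads stats from a data table, then teleports it to a given point or off-screen navmesh location and starts AIMoveTo with retry timers.
; Hits trigger knockback, red flash and floating text; death or lifespan expiry fades it out, then re-pools or destroys it.
; Bosses 16 and 31 add telegraphed projectiles, with 31 also speed-bursting.
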(event `SpawnSetup`
  (params (MonsterID :type Name) (RandomLocation :type Boolean) (SpecifiedLocation :type "Vector Structure") (`MoveToPlayer?` :type Boolean) (SpecificDestination :type "Vector Structure"))
  ;[0 0 0] Initialization
  (set `self.Monster ID` MonsterID)
  (set `self.Random Location` RandomLocation)
  (set `self.TeleportLocation` SpecifiedLocation)
  (set `self.ToPlayer?` `MoveToPlayer?`)
  (set `self.Destination` SpecificDestination)
  (bind _returnvalue (`|GetDataTableRow` (`self.DT_MonsterInfo`) (`self.Monster ID`))
    (:`then`
      (`CharacterMovementComponent.SetMovementMode` (`self.CharacterMovement`) "MOVE_None" 0)
      (bind (_id _name_ _flipbook _hp _atk _spd _exp _mass _droptreasurerate _lifespan _boss_) (break `/Game/_SG/Blueprints/Structs/F_MonsterInfo` _returnvalue))
      (set `self.InfoName` _name_)
      (`PaperFlipbookComponent.SetFlipbook` (`self.PaperFlipbook`) _flipbook)
      (set `self.InfoHP` _hp)
      (set `self.InfoATK` _atk)
      (set `CharacterMovementComponent.MaxWalkSpeed` _spd (`self.CharacterMovement`))
      (set `self.InfoEXP` _exp)
      (set `self.InfoMass` _mass)
      (bind _returnvalue_2 (`KismetSystemLibrary.K2_SetTimerDelegate` (`|CreateDelegate` :!event `ResetStatusByTimer`) _lifespan))
      (set `self.Timer_ReturnToPool` _returnvalue_2)
      (`PrimitiveComponent.SetMaterial` (`self.PaperFlipbook`) 0 "/Paper2D/TranslucentUnlitSpriteMaterial.TranslucentUnlitSpriteMaterial")
      (bind _ftactor (`self.FTActor`)
        (:`then`
          (`self.SetActorHiddenInGame` _ftactor true) ; Hidden at default
        )
        (:`else`
          _))
      (`|ExecutionSequence`
        (:`then_0`
          (if _boss_
            (switch `string` (`KismetStringLibrary.Conv_IntToString` _id)
              (:`16`
                (bind _returnvalue_3 (`KismetSystemLibrary.K2_SetTimerDelegate` (`|CreateDelegate` :!event `Boss16`) 0.1 true))
                (set `self.TimerHandle_CheckDistance` _returnvalue_3))
              (:`31`
                (bind _returnvalue_4 (`KismetSystemLibrary.K2_SetTimerDelegate` (`|CreateDelegate` :!event `Boss31`) 0.1 true))
                (set `self.TimerHandle_CheckDistance` _returnvalue_4)
                (set `self.InitWalkSpeed` (`CharacterMovementComponent.MaxWalkSpeed` (`self.CharacterMovement`)))))))
        (:`then_1`
          (`self.StartMarching`))))))

(event `StartMarching`
  ;[0 0 0] Initialization
  (if (`self.Random Location`)
    (`KismetSystemLibrary.K2_SetTimer` null "CheckSpawnLocation" 0.3 true)
    (else
      (`self.K2_TeleportTo` (`self.TeleportLocation`))
      (`self.PoolingRevive` (`self.ToPlayer?`) (`self.Destination`)))))

(event `/Game/_SG/Blueprints/Interfaces/BPI_Combat.INT_HitHandle`
  (params (DamageCauser :type "Actor Object Reference") (Damage :type "Float (double-precision)") (Force :type Integer))
  (bind _monster_id (`self.Monster ID`))
  ;[0 0 0] Hit & Death
  (set `self.Damage Causer` DamageCauser)
  (set `self.ReceivedDamage` Damage)
  (set `self.ReceivedForce` Force)
  (bind _damage_causer (`self.Damage Causer`)
    (:`then`
      (bind _live_ (message `/Game/_SG/Blueprints/Interfaces/BPI_Combat.INT_GetDead` _damage_causer))
      (if (and _live_ (not (`self.Dead`)))
        (`/Game/_SG/Data/GI_SG.HitSound` (`/Game/_SG/Data/Flib_SG.Flib_GetGI`))
        (bind _output_get (set `self.CurrentHP` (- (`self.CurrentHP`) (`self.ReceivedDamage`))))
        (`self.HPDisplay` _output_get)
        (if (<= _output_get 0.0)
          (`self.PoolingPickups`)
          (`self.PoolingDeath` :!label _label)
          (`self.StopAnim`)
          (bind (_direction _alpha) (`Timeline|FadingOutEffect` :!via `PlayFromStart` :!label _label_2)
            (:`Update`
              (bind _mi_transparent (`self.MI_Transparent`)
                (:`then`
                  (`MaterialInstanceDynamic.SetScalarParameterValue` _mi_transparent "Disappear" _alpha))
                (:`else`
                  (bind _returnvalue (`PrimitiveComponent.CreateDynamicMaterialInstance` (`self.PaperFlipbook`) 0 "/Game/_SG/Misc/MI_ModifiedSpriteMat.MI_ModifiedSpriteMat" "None"))
                  (set `self.MI_Transparent` _returnvalue))))
            (:`Finished`
              (`KismetArrayLibrary.Array_RemoveItem` (`/Game/_SG/Blueprints/BPA/BPA_LevelManager.ActiveMobPool` (`/Game/_SG/Data/GI_SG.Ref_LevelManager` (`/Game/_SG/Data/Flib_SG.Flib_GetGI`))) self)
              (if (`self.Pooling?`)
                (bind _returnvalue_2 (`self.K2_TeleportTo` (0.0 0.0 -10000.0))) ; Back to location where it comes from
                (if _returnvalue_2
                  (set `self.MobState` "NewEnumerator2")
                  (`/Game/_SG/Blueprints/BPA/BPA_LevelManager.TryRespawnMoreMobs` (`/Game/_SG/Data/GI_SG.Ref_LevelManager` (`/Game/_SG/Data/Flib_SG.Flib_GetGI`))) ; Replenish mobs
                  (else
                    (`KismetSystemLibrary.PrintString` "Teleporting Failure When Die" true true (struct :`R` 1.0 :`G` 0.17943 :`A` 1.0) 60.0)))
                (else
                  (if (== (`self.Monster ID`) "31")
                    (`/Game/_SG/Blueprints/UI/UI_Layout.GameOverUI` (`/Game/_SG/Data/Flib_SG.Flib_GetLayout`) true))
                  (if (or (== _monster_id "31") (== _monster_id "16"))
                    (`KismetSystemLibrary.K2_ClearAndInvalidateTimerHandle` (`self.TimerHandle_CheckDistance`)))
                  (bind _indicator (`self.Indicator`)
                    (:`then`
                      (`self.K2_DestroyActor` _indicator))
                    (:`else`
                      _))
                  (`self.K2_DestroyActor`)))))
          (else
            (`self.HandleKnockBackAndColor` (`self.Damage Causer`) (`self.ReceivedForce`))
            (`self.HandleDamageTexts` (`self.ReceivedDamage`))))))
    (:`else`)))

(event `HPDisplay`
  (params (Value :type "Float (double-precision)"))
  ;[0 0 0] Hit & Death
)

(event `ResetStatusByTimer`
  ;[0 0 0] Hit & Death
  (goto _label_2 :!via `PlayFromStart`))

(event `ForceDeath`
  ;[0 0 0] Hit & Death
  (goto _label))

(event `self.CapsuleComponent.OnComponentBeginOverlap`
  (params (OverlappedComponent :type "PrimitiveComponent Object Reference") (OtherActor :type "Actor Object Reference") (OtherComp :type "PrimitiveComponent Object Reference") (OtherBodyIndex :type Integer) (bFromSweep :type Boolean) (SweepResult :type "HitResult Structure (by ref)"))
  ;[0 0 0] Attack
  (if (and (`KismetSystemLibrary.IsValid` OtherActor) (`self.ActorHasTag` OtherActor "player"))
    (set `self.DamagedActor` OtherActor)
    (bind _damagedactor (`self.DamagedActor` :!label _label_3)
      (:`then`
        (if (not (`self.Dead`))
          (message `/Game/_SG/Blueprints/Interfaces/BPI_Combat.INT_HitHandle` _damagedactor self (`self.InfoATK`) 0)
          (bind _returnvalue (`KismetSystemLibrary.K2_SetTimerDelegate` (`|CreateDelegate` :!event `TouchDamage`) 0.5 true)) ; If enemy is still touching player after 0.5 seconds,\napply damage to player character again.
          (set `self.Timer_HandleATK` _returnvalue)
          (else
            (`KismetSystemLibrary.K2_ClearAndInvalidateTimerHandle` (`self.Timer_HandleATK`) :!label _label_4))))
      (:`else`
        (goto _label_4)))))

(event `self.CapsuleComponent.OnComponentEndOverlap`
  (params (OverlappedComponent :type "PrimitiveComponent Object Reference") (OtherActor :type "Actor Object Reference") (OtherComp :type "PrimitiveComponent Object Reference") (OtherBodyIndex :type Integer))
  ;[0 0 0] Attack
  (if (and (`KismetSystemLibrary.IsValid` OtherActor) (`self.ActorHasTag` OtherActor "player"))
    (set `self.DamagedActor` null)))

(event `TouchDamage`
  ;[0 0 0] Attack
  (goto _label_3))

(event `self.ReceiveTick`
  (params (DeltaSeconds :type "Float (single-precision)"))
  ;[0 0 0] Movement
  (`self.HandleDirections`)
  (if (`self.Touched`)
    (`/Engine/EditorBlueprintResources/StandardMacros.DoOnce` false :!label _label_5
      (:`Completed`
        (set `self.Touched` false)
        (`self.MoveTo` (`self.ToPlayer?`) (`self.Destination`))))))

(event `ResetMoving`
  ;[0 0 0] Movement
  (set `self.Touched` true)
  (`KismetSystemLibrary.Delay` 1.0)
  (goto _label_5 :!via `Reset`))

(event `MoveTo`
  (params (`ToPlayer?` :type Boolean) (Destination :type "Vector Structure"))
  (bind _returnvalue_x (`KismetMathLibrary.BreakVector` (`self.K2_GetActorLocation`)))
  (bind _returnvalue (`GameplayStatics.GetPlayerCharacter` 0))
  ;[0 0 0] Movement
  (if `ToPlayer?`
    (`/Engine/EditorBlueprintResources/StandardMacros.IsValid` _returnvalue :!label _label_6
      (:`Is Valid`
        (`|AIMoveTo` self (0.0 0.0 0.0) _returnvalue
          (:`OnSuccess`
            (`KismetSystemLibrary.K2_ClearAndInvalidateTimerHandle` (`self.TimerHandle_RestartApproaching`))
            (`self.ResetMoving`) ; Touching player character again
            (goto _label_7 :!via `Reset`))
          (:`OnFail`
            (`/Engine/EditorBlueprintResources/StandardMacros.DoOnce` false :!label _label_7
              (:`Completed`
                (bind _returnvalue_2 (`KismetSystemLibrary.K2_SetTimerDelegate` (`|CreateDelegate` :!event `RestartApproaching`) 0.2 true)) ; If mob failed to move, try again after 0.2 seconds
                (set `self.TimerHandle_RestartApproaching` _returnvalue_2)
                (`self.K2_AddActorLocalOffset` (0.0 0.0 1.0))))))))
    (else
      (set `self.ToLeft` (>= _returnvalue_x (.x Destination)))
      (`|AIMoveTo` self Destination null 20.0 :!label _label_8
        (:`OnSuccess`
          (`KismetSystemLibrary.K2_ClearAndInvalidateTimerHandle` (`self.TimerHandle_RestartApproachingLocation`))
          (`KismetSystemLibrary.K2_ClearAndInvalidateTimerHandle` (`self.Timer_ReturnToPool`))
          (`self.ResetStatusByTimer`)
          (goto _label_9 :!via `Reset`))
        (:`OnFail`
          (`/Engine/EditorBlueprintResources/StandardMacros.DoOnce` false :!label _label_9
            (:`Completed`
              (bind _returnvalue_3 (`KismetSystemLibrary.K2_SetTimerDelegate` (`|CreateDelegate` :!event `RestartApproachingLocation`) 0.2 true))
              (set `self.TimerHandle_RestartApproachingLocation` _returnvalue_3))))))))

(event `RestartApproaching`
  ;[0 0 0] Movement
  (goto _label_6))

(event `RestartApproachingLocation`
  ;[0 0 0] Movement
  (goto _label_8))

(event `Boss16`
  (bind (_returnvalue_x _returnvalue_y) (`KismetMathLibrary.BreakVector` (`self.K2_GetActorLocation`)))
  (bind _returnvalue (`KismetMathLibrary.FindLookAtRotation` (`self.K2_GetActorLocation`) (`self.K2_GetActorLocation` (`GameplayStatics.GetPlayerCharacter` 0))))
  ;[0 0 0] BOSS
  (`/Engine/EditorBlueprintResources/StandardMacros.DoOnce` false :!label _label_10
    (:`Completed`
      (`KismetSystemLibrary.Delay` 1.0)
      (bind _returnvalue_2 (`|SpawnActorFromClass` "/Game/_SG/Blueprints/BPA/BOSS/BPA_Indicator.BPA_Indicator_C" (`KismetMathLibrary.MakeTransform` (`KismetMathLibrary.MakeVector` _returnvalue_x _returnvalue_y 10.0) (`KismetMathLibrary.MakeRotator` 0.0 0.0 (.yaw _returnvalue))) "AdjustIfPossibleButAlwaysSpawn" "MultiplyWithRoot" null null))
      (set `self.Indicator` _returnvalue_2)
      (set `self.PlayerTempRotZ` _returnvalue)
      (`KismetSystemLibrary.Delay` 1.0) ; Leave some time for player to react
      (`self.K2_DestroyActor` (`self.Indicator`))
      (`/Game/_SG/Blueprints/BPA/BPA_LevelManager.PoolingBullets` (`/Game/_SG/Data/GI_SG.Ref_LevelManager` (`/Game/_SG/Data/Flib_SG.Flib_GetGI`)) (`self.K2_GetActorLocation`) (4.0 4.0 4.0) 30.0 (* (`KismetMathLibrary.Conv_RotatorToVector` (`self.PlayerTempRotZ`)) 500) "player" self "/Game/_SG/Blueprints/BPA/BOSS/FB_BossBullet.FB_BossBullet" (5.0 5.0 5.0) 8.0 (struct :`Yaw` -180.0 :`Roll` -90.0))
      (`KismetSystemLibrary.Delay` 3.0)
      (`self.ResetBossDoOnce`))))

(event `Boss31`
  (bind (_returnvalue_x _returnvalue_y) (`KismetMathLibrary.BreakVector` (`self.K2_GetActorLocation`)))
  (bind (_returnvalue_x_2 _returnvalue_y_2) (`KismetMathLibrary.BreakVector` (`self.K2_GetActorLocation`)))
  (bind (_returnvalue_x_3 _returnvalue_y_3) (`KismetMathLibrary.BreakVector` (`self.K2_GetActorLocation` (`GameplayStatics.GetPlayerCharacter` 0))))
  ;[0 0 0] BOSS
  (`|ExecutionSequence`
    (:`then_0`
      (if (> (`self.GetDistanceTo` (`GameplayStatics.GetPlayerCharacter` 0) self) 200.0)
        (`/Engine/EditorBlueprintResources/StandardMacros.DoOnce` false :!label _label_11
          (:`Completed`
            (bind _returnvalue (`GameplayStatics.SpawnEmitterAttached` "/Game/StarterContent/Particles/P_Fire.P_Fire" (`self.CapsuleComponent`) "None" (0.0 0.0 -10.0) (struct :`Pitch` 90.0) (0.7 0.7 0.7))) ; Visual effect only
            (set `self.BossVFX` _returnvalue)
            (`KismetSystemLibrary.Delay` 0.2) ; Waiting for player to react
            (set `CharacterMovementComponent.MaxWalkSpeed` (* (`self.InitWalkSpeed`) 2.0) (`self.CharacterMovement`))
            (`PaperFlipbookComponent.SetFlipbook` (`self.PaperFlipbook`) "/Game/_SG/Assets/Mobs/Mob31/FB_Mob31_FastSpeed.FB_Mob31_FastSpeed")
            (`KismetSystemLibrary.Delay` 2.7) ; Duration
            (set `CharacterMovementComponent.MaxWalkSpeed` (`self.InitWalkSpeed`) (`self.CharacterMovement`))
            (`PaperFlipbookComponent.SetFlipbook` (`self.PaperFlipbook`) "/Game/_SG/Assets/Mobs/Mob31/FB_Mob31.FB_Mob31")
            (bind _bossvfx (`self.BossVFX`)
              (:`then`
                (`ActorComponent.K2_DestroyComponent` _bossvfx)
                (`self.ResetQuickMoving`))
              (:`else`))))))
    (:`then_1`
      (if (<= (`KismetMathLibrary.Abs` (- _returnvalue_y_3 _returnvalue_y_2)) 55.0)
        (`/Engine/EditorBlueprintResources/StandardMacros.DoOnce` false :!label _label_12
          (:`Completed`
            (`KismetSystemLibrary.Delay` 1.0)
            (bind _returnvalue_2 (`|SpawnActorFromClass` "/Game/_SG/Blueprints/BPA/BOSS/BPA_Indicator.BPA_Indicator_C" (`KismetMathLibrary.MakeTransform` (`KismetMathLibrary.MakeVector` _returnvalue_x _returnvalue_y 10.0) (struct) (1.8 1.8 1.8)) "AdjustIfPossibleButAlwaysSpawn" "MultiplyWithRoot" null null))
            (set `self.Indicator` _returnvalue_2)
            (`KismetSystemLibrary.Delay` 1.0) ; Leave some time for player to react
            (`self.K2_DestroyActor` (`self.Indicator`))
            (`/Game/_SG/Blueprints/BPA/BPA_LevelManager.PoolingBullets` (`/Game/_SG/Data/GI_SG.Ref_LevelManager` (`/Game/_SG/Data/Flib_SG.Flib_GetGI`)) (`self.K2_GetActorLocation`) (6.0 6.0 6.0) 40.0 (select `bool` (not (`self.ToLeft`)) :`false` (-350.0 0.0 0.0) :`true` (350.0 0.0 0.0) :!type "Vector Structure") "player" self "/Game/_SG/Blueprints/BPA/BOSS/FB_BossBullet.FB_BossBullet" (5.5 5.5 5.5) 8.0 (struct :`Yaw` -180.0 :`Roll` -90.0))
            (`KismetSystemLibrary.Delay` 3.0)
            (`self.ResetBossDoOnce`)))))))

(event `ResetBossDoOnce`
  ;[0 0 0] BOSS
  (`|ExecutionSequence`
    (:`then_0`
      (goto _label_10 :!via `Reset`))
    (:`then_1`
      (goto _label_12 :!via `Reset`))))

(event `ResetQuickMoving`
  ;[0 0 0] BOSS
  (goto _label_11 :!via `Reset`))

(fn `CheckSpawnLocation`
  (locals (L_SpawnLocation :type "Vector Structure" :default (0.0 0.0 0.0)))
  (bind _randomlocation (`NavigationSystemV1.K2_GetRandomLocationInNavigableRadius` (`self.K2_GetActorLocation` (`GameplayStatics.GetPlayerCharacter` 0)) 800.0 null null))
  (bind _output_get (set `local.L_SpawnLocation` _randomlocation))
  (if (not (`/Game/_SG/Data/Flib_SG.Flib_CheckWihtinScreen` _output_get))
    (bind _returnvalue (`self.K2_TeleportTo` (+ (`local.L_SpawnLocation`) (0.0 0.0 10.0))))
    (if _returnvalue
      (`KismetSystemLibrary.K2_ClearTimer` null "CheckSpawnLocation")
      (`self.PoolingRevive` (`self.ToPlayer?`) (`self.Destination`)))))

(fn `HandleDamageTexts`
  (params (ReceivedDamage :type "Float (double-precision)"))
  (bind _ftactor (`self.FTActor`)
    (:`then`
      (`self.SetActorHiddenInGame` _ftactor false))
    (:`else`
      (bind _returnvalue (`|SpawnActorFromClass` "/Game/_SG/Blueprints/BPA/BPA_FloatingText.BPA_FloatingText_C" (`KismetMathLibrary.MakeTransform` (`SceneComponent.K2_GetComponentLocation` (`self.PaperFlipbook`))) "Undefined" "MultiplyWithRoot" null null))
      (bind _output_get (set `self.FTActor` _returnvalue))
      (`self.K2_AttachToComponent` _output_get (`self.PaperFlipbook`) "None" "KeepWorld" "KeepWorld" "KeepWorld" true)))
  (`/Game/_SG/Blueprints/BPA/BPA_FloatingText.DisplayFloatingText` (`self.FTActor`) (`KismetTextLibrary.Conv_IntToText` (`KismetMathLibrary.FTrunc` ReceivedDamage) false false) (struct :`R` 1.0 :`G` 1.0 :`B` 1.0 :`A` 1.0)))

(fn `HandleDirections`
  (bind _returnvalue_x (`KismetMathLibrary.BreakVector` (`self.K2_GetActorLocation`)))
  (bind _returnvalue_x_2 (`KismetMathLibrary.BreakVector` (`self.K2_GetActorLocation` (`GameplayStatics.GetPlayerCharacter` 0))))
  (if (<= _returnvalue_x_2 _returnvalue_x)
    (`/Engine/EditorBlueprintResources/StandardMacros.DoOnce` false :!label _label
      (:`Completed`
        (set `self.ToLeft` true)
        (goto _label_2 :!via `Reset`)))
    (else
      (`/Engine/EditorBlueprintResources/StandardMacros.DoOnce` false :!label _label_2
        (:`Completed`
          (set `self.ToLeft` false)
          (goto _label :!via `Reset`))))))

(fn `HandleKnockBackAndColor`
  (params (DamageCauser :type "Actor Object Reference") (ReceivedForce :type Integer))
  (`/Engine/EditorBlueprintResources/StandardMacros.IsValid` DamageCauser
    (:`Is Valid`
      (if (!= ReceivedForce 0)
        (`MovementComponent.StopMovementImmediately` (`self.CharacterMovement`))
        (`TimelineComponent.PlayFromStart` (`self.TL_Knockback`)))
      (`PaperFlipbookComponent.SetSpriteColor` (`self.PaperFlipbook`) (struct :`R` 1.0 :`A` 1.0))
      (`KismetSystemLibrary.K2_SetTimer` null "ResetColorAndMovement" 0.2))))

(fn `INT_GetDead`
  (returns (`Live?` :type Boolean))
  (return (not (`self.Dead`))))

(fn `OnRep_ToLeft`
  (bind _paperflipbook (`self.PaperFlipbook`))
  (if (`self.ToLeft`)
    (`SceneComponent.K2_SetWorldRotation` _paperflipbook (struct :`Yaw` 180.0 :`Roll` 90.0) false false)
    (else
      (`SceneComponent.K2_SetWorldRotation` _paperflipbook (struct :`Roll` -90.0) false false))))

(fn `PoolingDeath`
  (bind _capsulecomponent (`self.CapsuleComponent`))
  (set `self.DamagedActor` null)
  (set `self.Dead` true)
  (message `/Game/_SG/Blueprints/Interfaces/BPI_Interaction.INT_TriggerKilling` (`GameplayStatics.GetPlayerCharacter` 0))
  (`PrimitiveComponent.SetCollisionResponseToChannel` _capsulecomponent "ECC_Pawn" "ECR_Ignore")
  (`PrimitiveComponent.SetCollisionObjectType` _capsulecomponent "ECC_WorldDynamic")
  (`self.SetActorTickEnabled` false)
  (`CharacterMovementComponent.SetMovementMode` (`self.CharacterMovement`) "MOVE_None" 0)
  (`KismetSystemLibrary.K2_ClearAndInvalidateTimerHandle` (`self.Timer_HandleATK`))
  (`KismetSystemLibrary.K2_ClearAndInvalidateTimerHandle` (`self.Timer_ReturnToPool`))
  (`KismetSystemLibrary.K2_ClearAndInvalidateTimerHandle` (`self.TimerHandle_RestartApproaching`))
  (`KismetSystemLibrary.K2_ClearAndInvalidateTimerHandle` (`self.TimerHandle_RestartApproachingLocation`)))

(fn `PoolingPickups`
  (if (`KismetMathLibrary.RandomBoolWithWeight` 0.005)
    (`/Game/_SG/Blueprints/BPA/BPA_LevelManager.PoolingPickupBase` (`/Game/_SG/Data/GI_SG.Ref_LevelManager` (`/Game/_SG/Data/Flib_SG.Flib_GetGI`)) "NewEnumerator3" (`self.K2_GetActorLocation`) 0.0)
    (else
      (`/Game/_SG/Blueprints/BPA/BPA_LevelManager.PoolingPickupBase` (`/Game/_SG/Data/GI_SG.Ref_LevelManager` (`/Game/_SG/Data/Flib_SG.Flib_GetGI`)) "NewEnumerator1" (`self.K2_GetActorLocation`) (`self.InfoEXP`)))))

(fn `PoolingRevive`
  (params (`MoveToPlayer?` :type Boolean) (Destination :type "Vector Structure"))
  (bind _capsulecomponent (`self.CapsuleComponent`))
  (`|ExecutionSequence`
    (:`then_0`
      (set `self.Dead` false)
      (set `self.CurrentHP` (`self.InfoHP`))
      (`PrimitiveComponent.SetCollisionResponseToChannel` _capsulecomponent "ECC_Pawn" "ECR_Overlap")
      (`PrimitiveComponent.SetCollisionObjectType` _capsulecomponent "ECC_Pawn")
      (`CharacterMovementComponent.SetMovementMode` (`self.CharacterMovement`) "MOVE_Walking" 0))
    (:`then_1`
      (`self.SetActorTickEnabled` `MoveToPlayer?`) ; Tick is needed only when enemy runs to player
      (`self.MoveTo` `MoveToPlayer?` Destination)
      (`PrimitiveComponent.SetMaterial` (`self.PaperFlipbook`) 0 "/Paper2D/TranslucentUnlitSpriteMaterial.TranslucentUnlitSpriteMaterial") ; Optional
      (set `self.MI_Transparent` null) ; Set it to NULL
      (set `self.MobState` "NewEnumerator1"))))

(fn `ResetColorAndMovement`
  (`PaperFlipbookComponent.SetSpriteColor` (`self.PaperFlipbook`) (struct :`R` 1.0 :`G` 1.0 :`B` 1.0 :`A` 1.0))
  ;[0 0 0] Move to player character again
  (`self.MoveTo` (`self.ToPlayer?`) (`self.Destination`)))

(fn `StopAnim`
  (bind _ftactor (`self.FTActor`)
    (:`then`
      (`/Game/_SG/Blueprints/BPA/BPA_FloatingText.StopAnim` _ftactor)
      (`self.SetActorHiddenInGame` _ftactor true))
    (:`else`)))

(fn `UserConstructionScript`)
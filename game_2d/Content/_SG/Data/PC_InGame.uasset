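; PC_InGame is the in-game player controller that sets up the main UI.
; On BeginPlay it registers itself on the game instance as RefPCInGame, then creates the UI_Layout widget, adds it to the viewport and sets Game-and-UI input focused on it.
; Pressing F10 creates and shows a new UI_Options widget each time.
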(event `self.ReceiveBeginPlay`
  (set `/Game/_SG/Data/GI_SG.Ref_PCInGame` self (`/Game/_SG/Data/Flib_SG.Flib_GetGI`))
  (`self.CreateLayout`))

(event `Key|F10`
  (params (Key :type "Key Structure"))
  (:`Pressed`
    (bind _returnvalue (`|CreateWidget` "/Game/_SG/Blueprints/UI/UI_Options.UI_Options_C"))
    (`UserWidget.AddToViewport` _returnvalue 0)))

(fn `CreateLayout`
  (bind _returnvalue (`|CreateWidget` "/Game/_SG/Blueprints/UI/UI_Layout.UI_Layout_C"))
  (bind _output_get (set `self.UI_Layout` _returnvalue))
  (`UserWidget.AddToViewport` _output_get 0)
  (`WidgetBlueprintLibrary.SetInputMode_GameAndUIEx` self (`self.UI_Layout`)))

(fn `UserConstructionScript`)
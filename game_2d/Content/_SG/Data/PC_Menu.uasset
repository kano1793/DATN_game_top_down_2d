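; Player controller for the main menu that shows the mouse cursor and picks the first screen on BeginPlay.
; If the leaderboard is already initialized, it opens the menu, then after a short delay refreshes PlayFab via the saved player name, checks the save and loads data.
; Otherwise, an existing save triggers a GameInstance callback binding and data load.
; With no save, it shows the player name registration widget.
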(event `self.ReceiveBeginPlay`
  (bind _gi (`/Game/_SG/Data/Flib_SG.Flib_GetGI`))
  (bind _gi_2 (`/Game/_SG/Data/Flib_SG.Flib_GetGI`))
  ;[0 0 0] Show Register UI at the very beginning
  (set `self.bShowMouseCursor` true)
  (if (`/Game/_SG/Data/GI_SG.LeaderboardInit` _gi)
    (`self.CreateMenuUI`)
    ;;[0 0 0] Refresh Leaderboard
    (`KismetSystemLibrary.Delay` 0.2)
    (`/Game/_SG/Data/GI_SG.CreatePlayFabAccountBasedOnName` _gi_2 (`KismetTextLibrary.Conv_StringToText` (`/Game/_SG/Data/Saves/GSave_Gameplay.PlayerName` (`/Game/_SG/Data/GI_SG.Ref_SaveGameplay` _gi_2))))
    (`/Game/_SG/Data/GI_SG.CheckSave` _gi_2)
    (`/Game/_SG/Data/GI_SG.LoadData` _gi_2 :!label _label)
    (else
      (bind _returnvalue (`GameplayStatics.DoesSaveGameExist` (`/Game/_SG/Data/GI_SG.SaveSlots` _gi)))
      (if _returnvalue
        (add `/Game/_SG/Data/GI_SG.OnContinuousMenu` _gi_2 (`|CreateDelegate` :!event `CreateMenuUI`))
        (goto _label)
        (else
          (bind _returnvalue_2 (`|CreateWidget` "/Game/_SG/Blueprints/UI/UI_RegisterPlayerName.UI_RegisterPlayerName_C"))
          (`UserWidget.AddToViewport` _returnvalue_2 0)
          (`WidgetBlueprintLibrary.SetInputMode_GameAndUIEx` self _returnvalue_2 "DoNotLock" false))))))

(event `CreateMenuUI`
  ;[0 0 0] Show Register UI at the very beginning
  (bind _returnvalue (`|CreateWidget` "/Game/_SG/Blueprints/UI/UI_Menu.UI_Menu_C"))
  (bind _output_get (set `self.UI_Menu` _returnvalue))
  (`UserWidget.AddToViewport` _output_get 0)
  (`WidgetBlueprintLibrary.SetInputMode_GameAndUIEx` self _output_get "DoNotLock" false))

(fn `UserConstructionScript`)